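; BP_Grenade is a thrown grenade actor that explodes on a timer.
; On BeginPlay it applies a forward impulse to its Sphere, scaled by the Player's ChargeTime.
; After a three-second delay it runs a sphere trace for pawns and physics bodies, spawns an explosion emitter and destroys itself.
; The trace results are unused, so the blast applies no damage or force, and LaunchSpeed is also unused.
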(event `self.ReceiveBeginPlay`
  (bind _returnvalue (`SceneComponent.K2_GetComponentLocation` (`self.Sphere`)))
  (`PrimitiveComponent.AddImpulse` (`self.Sphere`) (* (* (`self.GetActorForwardVector`) 300.0) (+ (`/Game/FirstPerson/Blueprints/BP_FirstPersonCharacter.ChargeTime` (`self.Player`)) 1.0)) "None" false)
  (`KismetSystemLibrary.Delay` 3.0)
  (`KismetSystemLibrary.SphereTraceSingleForObjects` _returnvalue _returnvalue 10.0 (`|MakeArray` "ObjectTypeQuery3" "ObjectTypeQuery4" :!type "EObjectTypeQuery Enum") false (`|MakeArray` self :!type "Actor Object Reference"))
  (`GameplayStatics.SpawnEmitterAtLocation` "/Game/StarterContent/Particles/P_Explosion.P_Explosion" _returnvalue (struct) (10.0 10.0 10.0))
  (`self.K2_DestroyActor`))

(fn `UserConstructionScript`)