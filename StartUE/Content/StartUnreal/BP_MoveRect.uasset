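; BP_MoveRect is an actor that moves its Cube component around a 100-unit square in the relative XZ plane.
; While IsRun is set, Tick switches on MoveType (Right, Up, Left, Down), stepping one shared coordinate by one unit per frame, independent of delta time.
; DoPlay and DoStop extend parent versions, and both set IsRun to true, so DoStop does not halt the movement here.
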(event `self.ReceiveTick`
  (params (DeltaSeconds :type "Float (single-precision)"))
  (if (`self.IsRun`)
    (switch `/Game/StartUnreal/EN_MoveType` (`self.MoveType`)
      (:`NewEnumerator0`
        ;[1 1 1] 오른쪽 이동
        (bind _output_get (set `self.거기` (+ (`self.거기`) 1.0)))
        (`SceneComponent.K2_SetRelativeLocation` (`self.Cube`) (`KismetMathLibrary.MakeVector` _output_get) false false)
        (if (> (`self.거기`) 100.0)
          (set `self.MoveType` "NewEnumerator1")
          (set `self.거기` 0.0)))
      (:`NewEnumerator1`
        ;[1 1 1] 위쪽 이동
        (bind _output_get_2 (set `self.거기` (+ (`self.거기`) 1.0)))
        (`SceneComponent.K2_SetRelativeLocation` (`self.Cube`) (`KismetMathLibrary.MakeVector` 100.0 0.0 _output_get_2) false false)
        (if (> (`self.거기`) 100.0)
          (set `self.MoveType` "NewEnumerator2")))
      (:`NewEnumerator2`
        ;[1 1 1] 왼쪽 이동
        (bind _output_get_3 (set `self.거기` (- (`self.거기`) 1.0)))
        (`SceneComponent.K2_SetRelativeLocation` (`self.Cube`) (`KismetMathLibrary.MakeVector` _output_get_3 0.0 100.0) false false)
        (if (< (`self.거기`) 0.0)
          (set `self.MoveType` "NewEnumerator3")
          (set `self.거기` 100.0)))
      (:`NewEnumerator3`
        ;[1 1 1] 아래 이동
        (bind _output_get_4 (set `self.거기` (- (`self.거기`) 1.0)))
        (`SceneComponent.K2_SetRelativeLocation` (`self.Cube`) (`KismetMathLibrary.MakeVector` 0.0 0.0 _output_get_4) false false)
        (if (< (`self.거기`) 0.0)
          (set `self.MoveType` "NewEnumerator0"))))))

(fn `Do Play`
  (`parent.Do Play`)
  (set `self.IsRun` true))

(fn `Do Stop`
  (`parent.Do Stop`)
  (set `self.IsRun` true))

(fn `UserConstructionScript`)