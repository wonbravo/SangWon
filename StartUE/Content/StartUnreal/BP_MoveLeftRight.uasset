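; BP_MoveLeftRight is an actor that slides its Sphere back and forth along the local X axis.
; Each Tick steps an offset by a fixed, frame-dependent amount and sets the Sphere's relative location, flipping direction at either end of the range.
; An EventComponent's DoPlay and DoStop dispatchers start and pause the motion through the IsPlay flag.
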(event `self.ReceiveTick`
  (params (DeltaSeconds :type "Float (single-precision)"))
  (if (`self.IsPlay`)
    (if (`self.IsMoveRight`)
      ;[1 1 1] 오른쪽 이동
      (set `self.거기` (+ (`self.거기`) 1.0))
      (`SceneComponent.K2_SetRelativeLocation` (`self.Sphere`) (`KismetMathLibrary.MakeVector` (`self.거기`)) false false)
      (if (> (`self.거기`) 100.0)
        (set `self.IsMoveRight` false))
      (else
        ;[1 1 1] 왼쪽 이동
        (set `self.거기` (- (`self.거기`) 1.0))
        (`SceneComponent.K2_SetRelativeLocation` (`self.Sphere`) (`KismetMathLibrary.MakeVector` (`self.거기`)) false false)
        (if (< (`self.거기`) 0.0)
          (set `self.IsMoveRight` true))))))

(event `self.EventComponent.EventDispatcher_DoPlay`
  (set `self.IsPlay` true))

(event `self.EventComponent.EventDispatcher_DoStop`
  (set `self.IsPlay` false))

(fn `UserConstructionScript`)